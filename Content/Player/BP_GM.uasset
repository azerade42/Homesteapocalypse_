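; BP_GM is the game manager Blueprint that handles score, wave data, HUD, respawns and game over.
; BeginPlay resets score, creates the HUD and generates ten waves whose enemy count scales linearly with wave number.
; Respawn refills health and removes a HUD life; GameOver also hides the player, stops firing and opens a UI-only end screen.
; LoadScore, SaveScore and UpdateEnemyCount are empty stubs, and CamShake wraps world camera shake.
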(event Custom|UpdateEnemyCount
  (params (Count :type Integer)))

(event EventBeginPlay
  (CallFunction|LoadScore)
  (CallFunction|SetScore)
  (bind _returnvalue (UserInterface|CreateWidget "/Game/GUI/HUD.HUD_C"))
  (bind _output_get (Variables|Default|SetHUD _returnvalue))
  (UserInterface|Viewport|AddtoViewport _output_get 0)
  (for _index (range 1 10)
    (bind _output_get_2 (Variables|Default|SetIndex _index))
    (Utilities|Array|Add (Variables|Default|GetWAVE_DATA) (Utilities|Struct|MakeWaveData _output_get_2 (Math|Float|Truncate (* (Variables|Default|GetIndex) 3.0))))))

(event EventEndPlay
  (params (EndPlayReason :type EEndPlayReason%20Enum :default "Destroyed"))
  (CallFunction|SaveScore))

(fn ConstructionScript)

(fn LoadScore)

(fn SaveScore)

(fn SetScore
  (params (Score :type Integer))
  (bind _output_get (Variables|Default|SetScore (+ (Variables|Default|GetScore) Score)))
  (if (>= _output_get (Variables|Default|GetTopScore))
    (Variables|Default|SetTopScore _output_get)
    (else
      (Variables|Default|SetTopScore (Variables|Default|GetTopScore)))))

(fn CamShake
  (params (Shake :type Camera%20Shake%20Class%20Reference) (Epicenter :type Vector))
  (Camera|PlayWorldCameraShake Shake Epicenter 0.0 0.0))

(fn GameOver
  (bind _returnvalue (Game|GetPlayerController 0))
  (bind _returnvalue_2 (Game|Player|GetPlayerPawn 0))
  (Utilities|IsValid _returnvalue_2
    (:Is%20Valid
      (bind _asplayer_character (Utilities|Casting|CastToPlayerCharacter _returnvalue_2)
        (:then
          (Rendering|SetVisibility (Variables|/Game/Player/PlayerCharacter.PlayerCharacter_C|GetPlayerCharacter _asplayer_character) false true)
          (Utilities|Time|ClearTimerbyFunctionName _asplayer_character "Fire"))
        (:CastFailed
          _)))
    (:Is%20Not%20Valid
      _))
  (Default|RemoveLife (Variables|Default|GetHUD))
  (bind _returnvalue_3 (UserInterface|CreateWidget "/Game/GUI/GameOver.GameOver_C"))
  (UserInterface|Viewport|AddtoViewport _returnvalue_3 0)
  (Variables|/Script/Engine.PlayerController|SetbShowMouseCursor _returnvalue true)
  (Input|SetInputModeUIOnly _returnvalue _returnvalue_3 "DoNotLock"))

(fn Respawn
  (params (NewParam :type Player%20Character%20Object%20Reference))
  (Variables|/Game/Player/PlayerCharacter.PlayerCharacter_C|SetHealth NewParam (Variables|/Game/Player/PlayerCharacter.PlayerCharacter_C|GetMaxHealth NewParam))
  (Default|RemoveLife (Variables|Default|GetHUD)))